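; BP_Leech is an enemy that flies around a manager actor, falls, crawls toward the player, shoots projectiles and does arcing rushes.
; Movement is hand-coded: interpolated steering with trace-based avoidance in flight, plus ground traces, manual gravity and leech-to-leech separation on foot.
; Shootable and Rushable set attack flags from range and cooldown, timed by a clock advanced on Tick.
; Tick only updates that clock; no behavior function is called within this graph.
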(event EventBeginPlay
  (bind _flymanagerref (Variables|Fly|GetFlyManagerRef))
  (Utilities|IsValid _flymanagerref
    (:Is%20Valid
      (Transformation|SetActorLocation (+ (Transformation|GetActorLocation _flymanagerref) (Variables|Fly|GetOffsetLocal)) false false)
      (Utilities|FlowControl|Delay 0.1)
      (bind _outactors (Actor|GetAllActorsOfClass "BP_Leech_C"))
      (Variables|Fly|SetIgnoreLT _outactors))))

(event Collision|EventActorBeginOverlap
  (params (OtherActor :type Actor%20Object%20Reference)))

(event EventTick
  (params (DeltaSeconds :type Float%20%28single-precision%29))
  (CallFunction|TimeUpdate DeltaSeconds))

(fn ConstructionScript)

(fn StartFall
  ;[0.15 0.15 0.15 0.5] 이후 충격량 계산해서 초기 속도(Velocity) 여기다 설정 (Fall Tick도 수정 필요)
  (Variables|Fall|SetIsFalling true))

(fn FallTick
  (bind _returnvalue (Utilities|Time|GetWorldDeltaSeconds))
  (bind _returnvalue_2 (Transformation|GetActorLocation))
  (bind _output_get (Variables|Fall|SetFallVelocity (Math|Float|Max(Float) (+ (Variables|Fall|GetFallVelocity) (* (Variables|Fall|GetGravity) _returnvalue)) (Variables|Fall|GetTerminalVelocity))))
  (bind _sweephitresult (Transformation|SetActorLocation (Math|Vector|MakeVector (.x _returnvalue_2) (.y _returnvalue_2) (+ (* _output_get _returnvalue) (.z _returnvalue_2))) true false))
  (if (and (.bBlockingHit (Collision|BreakHitResult _sweephitresult)) (>= (.z (.ImpactNormal (Collision|BreakHitResult _sweephitresult))) 0.6))
    (Utilities|Casting|CastToBP_Leech (.HitActor (Collision|BreakHitResult _sweephitresult))
      (:CastFailed
        (Variables|Fall|SetIsFalling false)
        (Variables|Fall|SetFallVelocity 0.0)))))

(fn FlyTick
  (bind _returnvalue (Utilities|Time|GetWorldDeltaSeconds))
  (bind _returnvalue_2 (Transformation|GetActorLocation))
  (Utilities|IsValid (Variables|Fly|GetFlyManagerRef)
    (:Is%20Valid
      (bind (_outhit _returnvalue_3) (Collision|LineTraceByChannel _returnvalue_2 (+ _returnvalue_2 (* (Transformation|GetActorForwardVector) (Variables|Fly|GetAvoidDistance))) "TraceTypeQuery1" false (Variables|Fly|GetIgnoreLT) "None"))
      (if _returnvalue_3
        (Variables|Fly|SetAvoiddir (+ (Transformation|GetActorForwardVector) (* (.ImpactNormal (Collision|BreakHitResult _outhit)) (Variables|Fly|GetAvoidStrength))))
        (else
          (Variables|Fly|SetAvoiddir "0, 0, 0")))
      (bind _output_get (Variables|Fly|SetDesireVel (* (Math|Vector|Normalize (+ (Variables|Fly|GetAvoiddir) (Math|Vector|Normalize (- (+ (Transformation|GetActorLocation (Variables|Fly|GetFlyManagerRef)) (Variables|Fly|GetOffsetLocal)) (Transformation|GetActorLocation))))) (Variables|Fly|GetFlySpeed))))
      (bind _output_get_2 (Variables|Fly|SetVelocity (Math|Interpolation|VInterpTo (Variables|Fly|GetVelocity) _output_get _returnvalue (Variables|Fly|GetTurnRate))))
      (Transformation|SetActorLocation (+ (Transformation|GetActorLocation) (* _output_get_2 _returnvalue)) false false)
      (Transformation|SetWorldRotation (Variables|Default|GetCollision) (Math|Interpolation|RInterpTo (Transformation|GetActorRotation) (Math|Rotator|MakeRotfromX (Variables|Fly|GetVelocity)) (Utilities|Time|GetWorldDeltaSeconds) 1e+01) false false))))

(fn MoveTick
  (bind _returnvalue (Transformation|GetActorLocation))
  (bind _returnvalue_2 (Game|Player|GetPlayerPawn 0))
  (bind _returnvalue_3 (Transformation|GetActorLocation))
  (bind _returnvalue_4 (Transformation|GetActorLocation _returnvalue_2))
  (bind _returnvalue_5 (- _returnvalue_4 _returnvalue_3))
  (for _array_element (Collision|GetOverlappingActors "BP_Leech_C" :!class /Script/Engine.Actor)
    (Utilities|IsValid _array_element
      (:Is%20Valid
        (if (not (== self _array_element))
          (Transformation|AddActorWorldOffset (* (Math|Vector|Normalize (Math|Vector|MakeVector (.x (- (Transformation|GetActorLocation) (Transformation|GetActorLocation _array_element))) (.y (- (Transformation|GetActorLocation) (Transformation|GetActorLocation _array_element))) 0.0)) (Variables|Move|GetSeparationStrength) (Utilities|Time|GetWorldDeltaSeconds)))))))
  (Utilities|IsValid (Game|Player|GetPlayerPawn 0)
    (:Is%20Valid
      (bind (_outhit _returnvalue_6) (Collision|LineTraceByChannel _returnvalue (- _returnvalue (Math|Vector|MakeVector 0.0 0.0 (Variables|Move|GetGroundCheck))) "TraceTypeQuery1" false (Utilities|Array|MakeArray self) "None"))
      (if _returnvalue_6
        (Variables|Fall|SetFallVelocity 0.0)
        (bind _output_get (Variables|Move|SetLoc_Z (+ (.z (.Location (Collision|BreakHitResult _outhit))) 27.1)))
        (bind _output_get_2 (Variables|Fly|SetVelocity (Math|Vector|MakeVector (.x (Math|Interpolation|VInterpTo (Variables|Fly|GetVelocity) (* (Math|Vector|Normalize (Math|Vector|MakeVector (.x _returnvalue_5) (.y _returnvalue_5) 0.0)) (Variables|Move|GetMoveSpeed)) (Utilities|Time|GetWorldDeltaSeconds) (Variables|Fly|GetTurnRate))) (.y (Math|Interpolation|VInterpTo (Variables|Fly|GetVelocity) (* (Math|Vector|Normalize (Math|Vector|MakeVector (.x _returnvalue_5) (.y _returnvalue_5) 0.0)) (Variables|Move|GetMoveSpeed)) (Utilities|Time|GetWorldDeltaSeconds) (Variables|Fly|GetTurnRate))) (Variables|Fall|GetFallVelocity))))
        (Transformation|SetActorLocation (Math|Vector|MakeVector (.x (+ (* _output_get_2 (Utilities|Time|GetWorldDeltaSeconds)) (Transformation|GetActorLocation))) (.y (+ (* _output_get_2 (Utilities|Time|GetWorldDeltaSeconds)) (Transformation|GetActorLocation))) _output_get) true false)
        (else
          (Variables|Fall|SetFallVelocity (Math|Float|Max(Float) (Variables|Fall|GetTerminalVelocity) (+ (Variables|Fall|GetFallVelocity) (* (Variables|Fall|GetGravity) (Utilities|Time|GetWorldDeltaSeconds)))))
          (bind _output_get_3 (Variables|Fly|SetVelocity (Math|Vector|MakeVector (.x (Math|Interpolation|VInterpTo (Variables|Fly|GetVelocity) (* (Math|Vector|Normalize (Math|Vector|MakeVector (.x _returnvalue_5) (.y _returnvalue_5) 0.0)) (Variables|Move|GetMoveSpeed)) (Utilities|Time|GetWorldDeltaSeconds) (Variables|Fly|GetTurnRate))) (.y (Math|Interpolation|VInterpTo (Variables|Fly|GetVelocity) (* (Math|Vector|Normalize (Math|Vector|MakeVector (.x _returnvalue_5) (.y _returnvalue_5) 0.0)) (Variables|Move|GetMoveSpeed)) (Utilities|Time|GetWorldDeltaSeconds) (Variables|Fly|GetTurnRate))) (Variables|Fall|GetFallVelocity))))
          (Transformation|SetActorLocation (+ (* _output_get_3 (Utilities|Time|GetWorldDeltaSeconds)) (Transformation|GetActorLocation)) true false)))
      (Transformation|SetWorldRotation (Variables|Default|GetCollision) (Math|Interpolation|RInterpTo (Transformation|GetActorRotation) (Math|Rotator|MakeRotfromX (Variables|Fly|GetVelocity)) (Utilities|Time|GetWorldDeltaSeconds) 1e+01) false false))))

(fn TimeUpdate
  (params (Delta%20Second :type Float%20%28double-precision%29))
  (Variables|State|SetCurrTime (+ Delta%20Second (Variables|State|GetCurrTime))))

(fn Shootable
  (params (Player :type Actor%20Object%20Reference))
  (Utilities|IsValid Player
    (:Is%20Valid
      (Variables|Shoot|SetCanShoot (and (>= (Variables|Shoot|GetShootRange) (Math|Vector|VectorLength (- (Transformation|GetActorLocation Player) (Transformation|GetActorLocation)))) (> (- (Variables|State|GetCurrTime) (Variables|Shoot|GetShootTime)) (Variables|Shoot|GetShootCoolDown)))))))

(fn ShootTick
  (Game|SpawnActorfromClass "/Game/Cheon/Blueprints/BP_Leech_Projectile.BP_Leech_Projectile_C" (Transformation|GetWorldTransform (Variables|Default|GetLaunch)) "Undefined" "MultiplyWithRoot" 0 0)
  (Variables|Shoot|SetShootTime (Variables|State|GetCurrTime))
  (Variables|Shoot|SetCanShoot false))

(fn Rushable
  (params (Player :type Actor%20Object%20Reference))
  (bind _returnvalue (Transformation|GetActorLocation))
  (bind _returnvalue_2 (Transformation|GetActorLocation Player))
  (bind _returnvalue_3 (- _returnvalue_2 _returnvalue))
  (Utilities|IsValid Player
    (:Is%20Valid
      (Variables|Rush|SetCanRush (and (<= (Math|Vector|VectorLength (Math|Vector|MakeVector (.x _returnvalue_3) (.y _returnvalue_3) 0.0)) (Variables|Rush|GetRushRange)) (> (- (Variables|State|GetCurrTime) (Variables|Rush|GetRushCool)) 2.0))))))

(fn RushTick
  (bind _returnvalue (Utilities|Time|GetWorldDeltaSeconds))
  (if (Variables|Rush|GetIsRushing)
    (Variables|Rush|SetRushTime (+ (Variables|Rush|GetRushTime) _returnvalue))
    (bind _output_get (Variables|Rush|SetRushSpeedV (Math|Float|Max(Float) (+ (Variables|Rush|GetRushSpeedV) (* _returnvalue (Variables|Fall|GetGravity))) (Variables|Fall|GetTerminalVelocity))))
    (bind _output_get_2 (Variables|Rush|SetRushVelocity (Math|Vector|MakeVector (.x (Variables|Rush|GetRushVelocity)) (.y (Variables|Rush|GetRushVelocity)) _output_get)))
    (bind _sweephitresult (Transformation|AddActorWorldOffset (* _output_get_2 (Utilities|Time|GetWorldDeltaSeconds)) true))
    (if (or (.bBlockingHit (Collision|BreakHitResult _sweephitresult)) (>= (Variables|Rush|GetRushTime) (Variables|Rush|GetRushDuration)))
      (Rush|RushEnd))))

(fn RushEnd
  (Variables|Rush|SetRushSpeedV 3e+02)
  (Variables|Rush|SetRushVelocity "0, 0, 0")
  (Variables|Rush|SetIsRushing false)
  (bind _output_get (Variables|Rush|SetRushTime 0.0))
  (Variables|Rush|SetRushCool (Variables|State|GetCurrTime))
  (Development|PrintString (Utilities|String|ToString(Float) _output_get)))

(fn RushStart
  (bind _returnvalue (Game|Player|GetPlayerPawn 0))
  (bind _returnvalue_2 (Transformation|GetActorLocation))
  (bind _rushspeedh (Variables|Rush|GetRushSpeedH))
  (bind _returnvalue_3 (Transformation|GetActorLocation _returnvalue))
  (bind _returnvalue_4 (- _returnvalue_3 _returnvalue_2))
  (bind _returnvalue_5 (Math|Vector2D|MakeVector2D (.x _returnvalue_4) (.y _returnvalue_4)))
  (bind _returnvalue_6 (Math|Vector2D|Normalize2D _returnvalue_5))
  (bind _returnvalue_7 (* _rushspeedh _returnvalue_6))
  (Variables|Rush|SetRushTime 0.0)
  (Variables|Rush|SetIsRushing true)
  (bind _output_get (Variables|Rush|SetRushVelocity (Math|Vector|MakeVector (.x _returnvalue_7) (.y _returnvalue_7) (Variables|Rush|GetRushSpeedV))))
  (Transformation|SetActorRotation (Math|Rotator|MakeRotfromXZ _output_get (Transformation|GetActorUpVector))))