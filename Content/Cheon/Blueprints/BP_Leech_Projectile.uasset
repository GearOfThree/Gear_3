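; BP_Leech_Projectile is a lobbed projectile that flies toward the player's position at spawn, with no homing.
; BeginPlay sets a fixed horizontal velocity toward the player pawn, or destroys the projectile without one.
; Tick integrates gravity into vertical speed and moves it manually without sweep.
; Any actor overlap destroys it without applying damage; the gathered BP_Leech ignore list is never read and the hit event is empty.
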(event OnComponentHit(Collision)
  (params (HitComponent :type Primitive%20Component%20Object%20Reference) (OtherActor :type Actor%20Object%20Reference) (OtherComp :type Primitive%20Component%20Object%20Reference) (NormalImpulse :type Vector :default "0, 0, 0") (Hit :type Hit%20Result%20Structure%20%28by%20ref%29)))

(event EventBeginPlay
  (bind _returnvalue (Game|Player|GetPlayerPawn 0))
  (bind _returnvalue_2 (Transformation|GetActorLocation))
  (bind _returnvalue_3 (Transformation|GetActorLocation _returnvalue))
  (bind _returnvalue_4 (- _returnvalue_3 _returnvalue_2))
  (bind _outactors (Actor|GetAllActorsOfClass "/Game/Cheon/Blueprints/BP_Leech.BP_Leech_C"))
  (Variables|Default|SetIgnoreHit _outactors)
  (Utilities|IsValid _returnvalue
    (:Is%20Valid
      (Variables|Default|SetHorizontal%20Velo (* (Math|Vector|Normalize (Math|Vector|MakeVector (.x _returnvalue_4) (.y _returnvalue_4) 0.0)) (Variables|Default|GetHorizontal%20Speed))))
    (:Is%20Not%20Valid
      (Actor|DestroyActor))))

(event Collision|EventActorBeginOverlap
  (params (OtherActor :type Actor%20Object%20Reference))
  (Actor|DestroyActor))

(event EventTick
  (params (DeltaSeconds :type Float%20%28single-precision%29))
  (bind _horizontal_velo (Variables|Default|GetHorizontal%20Velo))
  (bind _output_get (Variables|Default|SetVertical%20Speed (+ (* DeltaSeconds (Variables|Default|GetGravity)) (Variables|Default|GetVertical%20Speed))))
  (bind _output_get_2 (Variables|Default|SetVelocity (Math|Vector|MakeVector (.x _horizontal_velo) (.y _horizontal_velo) _output_get)))
  (Transformation|SetActorLocation (+ (* _output_get_2 DeltaSeconds) (Transformation|GetActorLocation)) false false))

(fn ConstructionScript)