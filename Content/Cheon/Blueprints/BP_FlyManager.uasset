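; BP_FlyManager is an invisible-logic flock anchor that spawns a group of BP_Leech actors and wanders through the level.
; On BeginPlay it spawns one leech per Offsets entry, passing itself and that offset.
; Tick moves it at MaxSpeed without sweep, using a Delay to pick a random direction about every second.
; It steers back toward SpawnLoc when too far away or at MinVertical height or below.
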(event EventBeginPlay
  (for _index (range 0 (- (Utilities|Array|Length (Variables|Default|GetOffsets)) 1))
    (Game|SpawnActorfromClass "/Game/Cheon/Blueprints/BP_Leech.BP_Leech_C" (Transformation|GetActorTransform) "Undefined" "MultiplyWithRoot" 0 self (Utilities|Array|Get(acopy) (Variables|Default|GetOffsets) _index) 0)))

(event Collision|EventActorBeginOverlap
  (params (OtherActor :type Actor%20Object%20Reference)))

(event EventTick
  (params (DeltaSeconds :type Float%20%28single-precision%29))
  (Utilities|FlowControl|Sequence
    (:then_0
      (if (or (> (Math|Vector|VectorLength (- (Variables|Default|GetSpawnLoc) (Transformation|GetActorLocation))) 2.5e+03) (<= (.z (Transformation|GetActorLocation)) (Variables|Default|GetMin_Vertical)))
        (Variables|Default|SetDirection (Math|Vector|Normalize (- (Variables|Default|GetSpawnLoc) (Transformation|GetActorLocation))))
        (else
          (Utilities|FlowControl|Delay 1.0)
          (Variables|Default|SetDirection (Math|Random|RandomUnitVector)))))
    (:then_1
      (Transformation|SetActorLocation (+ (* (Variables|Default|GetMaxSpeed) (* DeltaSeconds (Variables|Default|GetDirection))) (Transformation|GetActorLocation)) false false))))

(fn ConstructionScript)